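; BP_Catch is a trigger that makes a robot arm react to thrown pickup cubes entering its reachable space.
; On overlap it counts the cube, gives it a short lifespan and passes joint rotations from ManipulateRobot to the Robot.
; ManipulateRobot uses the cube's world X, Y and Z directly as base yaw and two arm pitches, without inverse kinematics.
; Tick reloads the current level after a delay once three cubes have entered.
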(event `self.ReceiveActorBeginOverlap`
  (params (OtherActor :type "Actor Object Reference"))
  (bind _robot (`self.Robot`))
  ;[1 1 1] When thrown object overlaps robots reachable space, call manipulate robot to get new joint angles, then set those joint angles
  (bind _asbp_pickup_cube (cast `/Game/VirtualRealityBP/Blueprints/BP_PickupCube` OtherActor))
  (bind _result (`/Engine/EditorBlueprintResources/StandardMacros.IncrementInt` (`self.ThrownCubes`))
    (:`  `
      (set `self.ThrownCubes` _result)
      (`self.SetLifeSpan` _asbp_pickup_cube 3.0)
      (set `self.bGenerateOverlapEventsDuringLevelStreaming` false)
      (bind (_base _arm1 _arm2) (`self.ManipulateRobot` _asbp_pickup_cube))
      (`/Engine/EditorBlueprintResources/StandardMacros.IsValid` _robot
        (:`Is Valid`
          (`/Game/Robot_Model/BP_Robot.SetJointAngles` _robot _base _arm1 _arm2))))))

(event `self.ReceiveTick`
  (params (DeltaSeconds :type "Float (single-precision)"))
  ;[1 1 1] Check for all cubes thrown into space, then reload the world
  (if (== 3 (`self.ThrownCubes`))
    (`KismetSystemLibrary.Delay` 3.0)
    (bind _returnvalue (`GameplayStatics.GetCurrentLevelName` true))
    (`GameplayStatics.OpenLevel` (`KismetStringLibrary.Conv_StringToName` _returnvalue))))

(fn `ManipulateRobot`
  (params (Throwable :type "/Game/VirtualRealityBP/Blueprints/BP_PickupCube Object Reference"))
  (returns (Base :type "Rotator Structure") (Arm1 :type "Rotator Structure") (Arm2 :type "Rotator Structure"))
  (return (`KismetMathLibrary.MakeRotator` 0.0 0.0 (.x (`self.K2_GetActorLocation` Throwable))) (`KismetMathLibrary.MakeRotator` 0.0 (.y (`self.K2_GetActorLocation` Throwable))) (`KismetMathLibrary.MakeRotator` 0.0 (.z (`self.K2_GetActorLocation` Throwable)))))

(fn `UserConstructionScript`)